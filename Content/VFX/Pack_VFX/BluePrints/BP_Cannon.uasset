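; BP_Cannon is a repeating spawner in the VFX pack that launches actors of a configurable class.
; On BeginPlay it spawns one actor immediately and starts a looping Timeout timer at the TimeReplay interval, which spawns another on each tick of the timer.
; Each actor takes its location and forward-facing rotation from the SpawnREF component, at unit scale.
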(event `self.ReceiveBeginPlay`
  (bind _spawn_ref (`self.Spawn REF`))
  (`KismetSystemLibrary.K2_SetTimer` null "Timeout" (`self.Time_Replay`) true)
  (`|SpawnActorFromClass` (`self.BP`) (`KismetMathLibrary.MakeTransform` (`SceneComponent.K2_GetComponentLocation` _spawn_ref) (`KismetMathLibrary.Conv_VectorToRotator` (`SceneComponent.GetForwardVector` _spawn_ref))) "Undefined" "SelectDefaultAtRuntime" null null))

(event `Timeout`
  (bind _spawn_ref (`self.Spawn REF`))
  (`|SpawnActorFromClass` (`self.BP`) (`KismetMathLibrary.MakeTransform` (`SceneComponent.K2_GetComponentLocation` _spawn_ref) (`KismetMathLibrary.Conv_VectorToRotator` (`SceneComponent.GetForwardVector` _spawn_ref))) "Undefined" "SelectDefaultAtRuntime" null null))

(fn `UserConstructionScript`)