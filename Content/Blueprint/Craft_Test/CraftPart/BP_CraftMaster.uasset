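; BP_CraftMaster is a craftable object that materializes through a gradient effect when interacted with and shows an info widget.
; SetCraftMesh assigns the mesh, caches and overrides its materials, and makes it block only the Visibility channel.
; InteractwithCraft plays or stops a timeline driving the Gradient_Offset material parameter; on finish, cached materials and full collision return.
; LookAt displays a message through W_DisplayInfo, with widget visibility toggled separately.
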(event `self.ReceiveBeginPlay`
  (bind _asbp_building_character (cast `/Game/Blueprint/Character/Player/BP_BuildingCharacter` (`GameplayStatics.GetPlayerCharacter` 0)))
  (set `self.Player` _asbp_building_character)
  (`SceneComponent.SetHiddenInGame` (`self.Widget`) false false))

(event `self.SetCraftMesh`
  (params (CraftMesh :type "StaticMesh Object Reference"))
  (bind _craft (`self.Craft`))
  (bind _returnvalue (`MeshComponent.GetMaterials` (`self.Craft`)))
  (`StaticMeshComponent.SetStaticMesh` (`self.Craft`) CraftMesh)
  (set `self.Materials` _returnvalue)
  (for (_ _array_index) _returnvalue
    (`PrimitiveComponent.SetMaterial` _craft _array_index null)
    (if (not (`self.IsCraftFinished`))
      (`/Engine/EditorBlueprintResources/StandardMacros.IncrementInt` (`self.ResourcesPlaced`)
        (:`  `
          (if (== (`self.Cost`) (`self.ResourcesPlaced`))
            (set `self.IsCraftFinished` true))))))
  (`PrimitiveComponent.SetCollisionResponseToAllChannels` _craft "ECR_Ignore")
  (`PrimitiveComponent.SetCollisionResponseToChannel` _craft "ECC_Visibility" "ECR_Block"))

(event `self.SetCraftCost`
  (params (Resource :type Integer))
  (set `self.Cost` Resource))

(event `self.InteractWithCraft`
  (params (IsTrigger :type Boolean))
  (bind _craft (`self.Craft`))
  (if IsTrigger
    (bind (_direction _gradient) (`Timeline|GradientTimeline` :!label _label)
      (:`Update`
        (`MeshComponent.SetScalarParameterValueOnMaterials` _craft "Gradient_Offset" _gradient))
      (:`Finished`
        (for (_array_element _array_index) (`self.Materials`)
          (`PrimitiveComponent.SetMaterial` _craft _array_index _array_element))
        (`PrimitiveComponent.SetCollisionResponseToAllChannels` _craft "ECR_Block")
        (`PrimitiveComponent.SetCollisionResponseToChannel` _craft "ECC_Visibility" "ECR_Block")))
    (else
      (goto _label :!via `Stop`))))

(event `/Game/Blueprint/Component/Inventory/IInteractInterface.InteractWith`
  (params (PlayerCharacter :type "/Game/Blueprint/Character/Player/BP_PlayerCharacter Object Reference")))

(fn `LookAt`
  (returns (Message :type Text))
  (bind _asw_display_info (cast `/Game/Blueprint/Component/Inventory/UI/Base/W_DisplayInfo` (`WidgetComponent.GetWidget` (`self.Widget`))))
  (`/Game/Blueprint/Component/Inventory/UI/Base/W_DisplayInfo.ShowMessage` _asw_display_info (`self.Message`))
  (return ""))

(fn `Set Visibility Widget`
  (params (Result :type Boolean))
  (`SceneComponent.SetHiddenInGame` (`self.Widget`) Result false)
  (return))

(fn `UserConstructionScript`)