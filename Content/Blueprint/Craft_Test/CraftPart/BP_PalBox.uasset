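; BP_PalBox is an interactable Pal storage box that shows its contents in the player's HUD.
; On BeginPlay it fills its PalInventorySystem with one entry for every row of DT_PalData, each with a default profile struct.
; Interacting gets player controller 0 as BP_PlayerController and passes the inventory to its HUD's DisplayPalBox.
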(event `self.ReceiveBeginPlay`
  (bind _outrownames (`DataTableFunctionLibrary.GetDataTableRowNames` "/Game/Blueprint/Component/Inventory/DataTable/DT_PalData.DT_PalData"))
  (for _array_element _outrownames
    (`/Game/Blueprint/Component/Inventory/PalInventorySystem.Add to PalInventory` (`self.PalInventorySystem`) _array_element 1 (make `/Game/Blueprint/Component/Inventory/Struct/FPalProfileStruct` 1))))

(event `/Game/Blueprint/Component/Inventory/IInteractInterface.InteractWith`
  (params (PlayerCharacter :type "/Game/Blueprint/Character/Player/BP_PlayerCharacter Object Reference"))
  (bind _asbp_player_controller (cast `/Game/Blueprint/Character/Player/Controller/BP_PlayerController` (`GameplayStatics.GetPlayerController` 0)))
  (`/Game/Blueprint/Component/Inventory/UI/Base/W_PlayerHUD.DisplayPalBox` (`/Game/Blueprint/Character/Player/Controller/BP_PlayerController.HUD` _asbp_player_controller) (`self.PalInventorySystem`)))

(fn `UserConstructionScript`
  (`parent.UserConstructionScript`))