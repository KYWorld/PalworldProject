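; Game instance Blueprint that holds the player's character customization: head, hair and name.
; SaveCustomData stores the three values on the instance.
; SetCustomData applies the saved head and hair to a given player by setting skeletal mesh assets on its CharacterEquipmentMap entries, only when both are valid.
; The saved name is not applied there.
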(fn `SaveCustomData`
  (params (Head :type "SkeletalMesh Object Reference") (Hair :type "SkeletalMesh Object Reference") (Name :type Text))
  (set `self.Head` Head)
  (set `self.Hair` Hair)
  (set `self.Name` Name))

(fn `SetCustomData`
  (params (Player :type "/Game/Blueprint/Character/Player/BP_PlayerCharacter Object Reference"))
  (bind _characterequipmentmap (`PlayerCharacter.CharacterEquipmentMap` Player))
  (bind _head (`self.Head`)
    (:`then`
      (bind _hair (`self.Hair`)
        (:`then`
          (set `SkeletalMeshComponent.SkeletalMeshAsset` _head (`BlueprintMapLibrary.Map_Find` _characterequipmentmap "Head"))
          (set `SkeletalMeshComponent.SkeletalMeshAsset` _hair (`BlueprintMapLibrary.Map_Find` _characterequipmentmap "Hair")))
        (:`else`)))
    (:`else`)))