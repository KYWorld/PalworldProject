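; BP_HawkBird is the character Blueprint for the HawkBird Pal, filed under ground monsters.
; It enables actor tick on BeginPlay and leaves construction to its parent.
; The MoveToFly event adds movement input along control-rotation axes: forward uses yaw only, right uses yaw and roll, so pitch is ignored.
; Overlap and Tick events are empty, and LookAt returns an empty value.
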(event `self.ReceiveBeginPlay`
  (`self.SetActorTickEnabled` true))

(event `MoveToFly`
  (params (ValueX :type "Float (double-precision)") (ValueY :type "Float (double-precision)"))
  (bind (_returnvalue_roll _returnvalue_pitch _returnvalue_yaw) (`KismetMathLibrary.BreakRotator` (`self.GetControlRotation`)))
  (bind (_returnvalue_roll_2 _returnvalue_pitch_2 _returnvalue_yaw_2) (`KismetMathLibrary.BreakRotator` (`self.GetControlRotation`)))
  (`self.AddMovementInput` (`KismetMathLibrary.GetRightVector` (`KismetMathLibrary.MakeRotator` _returnvalue_roll_2 0.0 _returnvalue_yaw_2)) ValueX)
  (`self.AddMovementInput` (`KismetMathLibrary.GetForwardVector` (`KismetMathLibrary.MakeRotator` 0.0 0.0 _returnvalue_yaw)) ValueY))

(fn `LookAt`
  (returns (Message :type Text))
  (return ""))

(fn `UserConstructionScript`
  (`parent.UserConstructionScript`))