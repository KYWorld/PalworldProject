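; Base character for Pals: creatures with a profile, state, overhead info widget and self-only scene capture.
; SetState drives eye and mouth expressions through UV offsets on materials found by row name; Dead is final, stopping AI and enabling physics.
; Player overlaps on non-zero-team Pals send a HitReact gameplay event carrying calculated damage, with effects.
; Weight sets scale; experience drives data-table level-ups to level 10, refreshing HUD and widget.
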(event `self.ReceiveBeginPlay`
  (`SceneCaptureComponent.ShowOnlyActorComponents` (`self.SceneCaptureComponent2D`) self false))

(event `self.CapsuleComponent.OnComponentBeginOverlap`
  (params (OverlappedComponent :type "PrimitiveComponent Object Reference") (OtherActor :type "Actor Object Reference") (OtherComp :type "PrimitiveComponent Object Reference") (OtherBodyIndex :type Integer) (bFromSweep :type Boolean) (SweepResult :type "HitResult Structure (by ref)"))
  (bind _returnvalue (`SceneComponent.K2_GetComponentLocation` OtherComp))
  (bind _asbp_player_character (cast `/Game/Blueprint/Character/Player/BP_PlayerCharacter` OtherActor))
  (bind _asbp_base_aicontroller (cast `/Game/Blueprint/Character/Pal/BP_BaseAIController` (`self.GetController`)))
  (bind _returnvalue_2 (`BaseAIController.GetTeamId` _asbp_base_aicontroller))
  (if (!= (break `GenericTeamId` _returnvalue_2) 0)
    (bind (_currentplayerprofile_level _currentplayerprofile_exp _currentplayerprofile_hp _currentplayerprofile_stamina _currentplayerprofile_enengy _currentplayerprofile_attack _currentplayerprofile_defence _currentplayerprofile_weight _currentplayerprofile_workspeed _currentplayerprofile_weapondamage) (break `/Game/Blueprint/Component/Inventory/Struct/FPlayerProfileStruct` (`/Game/Blueprint/Character/Player/BP_PlayerCharacter.CurrentPlayerProfile` _asbp_player_character)))
    (`AbilitySystemBlueprintLibrary.SendGameplayEventToActor` self (struct :`TagName` "Shared.Event.HitReact") (make `GameplayEventData` (struct) _asbp_player_character self null null (struct) (struct) (struct) (`BaseFunctionLibrary.DamageCulculation` _currentplayerprofile_attack _currentplayerprofile_weapondamage)))
    (`GameplayStatics.SpawnEmitterAtLocation` "/Game/InsaneGunnerSet/demo/FX/P_Hit.P_Hit" _returnvalue)
    (`GameplayStatics.PlaySoundAtLocation` "/Game/PalworldAsset/Sound/UI/HitSound/AKE_Critical.AKE_Critical" _returnvalue (struct) 1.0 1.0 0.0 null null null null)))

(fn `AddExp`
  (params (Amount :type "Float (double-precision)"))
  (bind _profile (`self.Profile`))
  (bind (_level _gender _isboss _weight _attack _defence _workspeed _enengy _teamid _isspawn _currenthp _exp _maxhp _maxexp) (break `/Game/Blueprint/Component/Inventory/Struct/FPalProfileStruct` _profile))
  (bind _returnvalue (+ Amount _exp))
  (bind _structout (setmembers `/Game/Blueprint/Component/Inventory/Struct/FPalProfileStruct` :`StructRef` _profile :`Exp` _returnvalue))
  (set `self.Profile` _structout)
  (if (and (>= _returnvalue _maxexp) (< _level 10))
    (`self.LevelUp` (+ _level 1))
    (else
      (`self.Update Widget`))))

(fn `LevelUp`
  (params (Level :type Integer))
  (bind _profile (`self.Profile`))
  (bind (_level _gender _isboss _weight _attack _defence _workspeed _enengy _teamid _isspawn _currenthp _exp _maxhp _maxexp) (break `/Game/Blueprint/Component/Inventory/Struct/FPalProfileStruct` _profile))
  (bind _returnvalue (`|GetDataTableRow` "/Game/Blueprint/Component/Inventory/DataTable/DT_PalLevelData.DT_PalLevelData" (`KismetStringLibrary.Conv_StringToName` (`KismetStringLibrary.Conv_IntToString` Level)))
    (:`then`
      (bind (_level_2 _gender_2 _isboss_2 _weight_2 _attack_2 _defence_2 _workspeed_2 _enengy_2 _teamid_2 _isspawn_2 _currenthp_2 _exp_2 _maxhp_2 _maxexp_2) (break `/Game/Blueprint/Component/Inventory/Struct/FPalProfileStruct` _returnvalue))
      (bind _returnvalue_2 (+ _maxhp_2 _maxhp))
      (bind _structout (setmembers `/Game/Blueprint/Component/Inventory/Struct/FPalProfileStruct` :`StructRef` _profile :`Level` Level :`Attack` (+ _attack_2 _attack) :`Defence` (+ _defence_2 _defence) :`CurrentHp` _returnvalue_2 :`Exp` 0.0 :`MaxHp` _returnvalue_2 :`MaxExp` (+ _maxexp_2 _maxexp) :`MaxEnergy` 0.0))
      (set `self.Profile` _structout)
      (`self.Update Widget`))))

(fn `LookAt`
  (returns (Message :type Text))
  (bind (_itemid_datatable _itemid_rowname) (break `DataTableRowHandle` (`/Game/Blueprint/Component/Inventory/PalDataComponent.ItemID` (`self.PalDataComponent`))))
  (bind _returnvalue (`|GetDataTableRow` "/Game/Blueprint/Component/Inventory/DataTable/DT_PalData.DT_PalData" _itemid_rowname)
    (:`then`
      (bind _asw_pal_display_widget (cast `/Game/Blueprint/Component/Inventory/UI/W_PalDisplayWidget` (`WidgetComponent.GetWidget` (`self.Widget`))))
      (`/Game/Blueprint/Component/Inventory/UI/W_PalDisplayWidget.ShowPalDisplayInfo` _asw_pal_display_widget (`self.Profile`) _returnvalue)
      (return ""))))

(fn `Set Visibility Widget`
  (params (Result :type Boolean))
  (returns (NewParam :type Boolean))
  (`SceneComponent.SetHiddenInGame` (`self.Widget`) Result false)
  (return false))

(fn `SetState`
  (params (NewPalState :type "/Game/Blueprint/Enum/EPalState Enum" :default "NewEnumerator11"))
  (locals (NewLocalVar :type "GameplayTagContainer Structure"))
  (bind _mesh (`self.Mesh`))
  (bind _mesh_2 (`self.Mesh`))
  (bind (_itemid_datatable _itemid_rowname) (break `DataTableRowHandle` (`/Game/Blueprint/Component/Inventory/PalDataComponent.ItemID` (`self.PalDataComponent`))))
  (bind (_itemid_datatable_2 _itemid_rowname_2) (break `DataTableRowHandle` (`/Game/Blueprint/Component/Inventory/PalDataComponent.ItemID` (`self.PalDataComponent`))))
  (bind _returnvalue (`KismetStringLibrary.Conv_StringToName` (`KismetSystemLibrary.MakeLiteralString` (`KismetStringLibrary.Concat_StrStr` "MI_" (`KismetStringLibrary.Conv_NameToString` _itemid_rowname_2) "_Eye"))))
  (bind _returnvalue_2 (`KismetStringLibrary.Conv_StringToName` (`KismetSystemLibrary.MakeLiteralString` (`KismetStringLibrary.Concat_StrStr` "MI_" (`KismetStringLibrary.Conv_NameToString` _itemid_rowname) "_Mouth"))))
  (bind _returnvalue_3 (`PrimitiveComponent.GetMaterialByName` _mesh _returnvalue_2))
  (bind _returnvalue_4 (`PrimitiveComponent.GetMaterialByName` _mesh_2 _returnvalue))
  (if (not (`|EnumEquality` (`self.PalState`) "NewEnumerator18"))
    (set `self.PalState` NewPalState)
    (if (`|EnumEquality` (`self.PalState`) "NewEnumerator18")
      (`BrainComponent.StopLogic` (`AIController.BrainComponent` (`AIBlueprintHelperLibrary.GetAIController` self)) "")
      (`PrimitiveComponent.SetCollisionEnabled` (`self.CapsuleComponent`) "NoCollision")
      (`PrimitiveComponent.SetSimulatePhysics` (`self.Mesh`) true)
      (`PrimitiveComponent.SetSimulatePhysics` (`self.CapsuleComponent`) true)
      (`AbilitySystemBlueprintLibrary.AddLooseGameplayTags` self (`BlueprintGameplayTagLibrary.MakeLiteralGameplayTagContainer` (struct :`GameplayTags` (struct :`(TagName` "Player.Event.Death")))))
      (else
        (`/Engine/EditorBlueprintResources/StandardMacros.IsValid` _returnvalue_4
          (:`Is Valid`
            _))))
    (bind _returnvalue_5 (`PrimitiveComponent.CreateDynamicMaterialInstance` _mesh_2 (`PrimitiveComponent.GetMaterialIndex` _mesh_2 _returnvalue) _returnvalue_4 "None"))
    (`MaterialInstanceDynamic.SetScalarParameterValue` _returnvalue_5 "U" (select `/Game/Blueprint/Enum/EPalState` (`self.PalState`) :`NewEnumerator12` 0.5 :`NewEnumerator14` 0.5 :`NewEnumerator16` 0.5 :`NewEnumerator18` 0.5 :`NewEnumerator22` 0.5 :!type "Float (single-precision)"))
    (`MaterialInstanceDynamic.SetScalarParameterValue` _returnvalue_5 "V" (select `/Game/Blueprint/Enum/EPalState` (`self.PalState`) :`NewEnumerator13` 0.25 :`NewEnumerator14` 0.25 :`NewEnumerator15` 0.5 :`NewEnumerator16` 0.5 :`NewEnumerator17` 0.75 :`NewEnumerator18` 0.75 :`NewEnumerator20` 0.25 :`NewEnumerator22` 0.25 :!type "Float (single-precision)"))
    (`/Engine/EditorBlueprintResources/StandardMacros.IsValid` _returnvalue_3
      (:`Is Valid`
        (bind _returnvalue_6 (`PrimitiveComponent.CreateDynamicMaterialInstance` _mesh (`PrimitiveComponent.GetMaterialIndex` _mesh _returnvalue_2) _returnvalue_3 "None"))
        (`MaterialInstanceDynamic.SetScalarParameterValue` _returnvalue_6 "U" (select `/Game/Blueprint/Enum/EPalState` (`self.PalState`) :`NewEnumerator12` 0.5 :`NewEnumerator14` 0.5 :`NewEnumerator17` 0.5 :`NewEnumerator18` 0.5 :!type "Float (single-precision)"))
        (`MaterialInstanceDynamic.SetScalarParameterValue` _returnvalue_6 "V" (select `/Game/Blueprint/Enum/EPalState` (`self.PalState`) :`NewEnumerator14` 0.5 :`NewEnumerator16` 0.5 :`NewEnumerator17` 0.5 :`NewEnumerator18` 0.5 :!type "Float (single-precision)"))))))

(fn `Update Widget`
  (bind _asbp_player_controller (cast `/Game/Blueprint/Character/Player/Controller/BP_PlayerController` (`GameplayStatics.GetPlayerController` 0)))
  (`/Game/Blueprint/Component/Inventory/UI/W_HUD.SetData` (`/Game/Blueprint/Character/Player/Controller/BP_PlayerController.HUD` _asbp_player_controller))
  (`self.LookAt`))

(fn `UserConstructionScript`
  (bind (_profile_level _profile_gender _profile_isboss _profile_weight) (break `/Game/Blueprint/Component/Inventory/Struct/FPalProfileStruct` (`self.Profile`)))
  (`self.SetActorScale3D` (select `/Game/Blueprint/Enum/EPalWeight` _profile_weight :`NewEnumerator11` (0.5 0.5 0.5) :`NewEnumerator12` (1.0 1.0 1.0) :`NewEnumerator13` (1.5 1.5 1.5) :`NewEnumerator14` (3.0 3.0 3.0) :!type "Vector Structure"))
  (`self.SetState` "NewEnumerator11"))