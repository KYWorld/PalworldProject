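; Base AI controller for Pal characters that sets the team ID on possess and runs the friend or enemy behavior tree to match.
; AI perception keeps the nearer actor as the blackboard target, firing the Pal's encounter ability on first acquisition or when switching to a player.
; Forgetting the target clears it and changes the Pal's state.
; SetParentActor writes a parent actor to the blackboard.
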(event `self.ReceivePossess`
  (params (PossessedPawn :type "Pawn Object Reference"))
  (bind _asbp_pal_character_base (cast `/Game/Blueprint/Character/Pal/BP_PalCharacterBase` PossessedPawn))
  (set `self.Pal` _asbp_pal_character_base)
  (bind (_profile_level _profile_gender _profile_isboss _profile_weight _profile_attack _profile_defence _profile_workspeed _profile_enengy _profile_teamid) (break `/Game/Blueprint/Component/Inventory/Struct/FPalProfileStruct` (`/Game/Blueprint/Character/Pal/BP_PalCharacterBase.Profile` _asbp_pal_character_base)))
  (`self.SetTeamId` _profile_teamid)
  (bind _returnvalue (select `byte` (`.TeamID` (break `GenericTeamId` _profile_teamid)) :`0` (`self.FriendBTAsset`) :`1` (`self.EnemyBTAsset`)))
  (`/Engine/EditorBlueprintResources/StandardMacros.IsValid` _returnvalue
    (:`Is Valid`
      (`self.RunBehaviorTree` _returnvalue))))

(event `self.AIPerceptionComponent.OnTargetPerceptionUpdated`
  (params (Actor :type "Actor Object Reference") (Stimulus :type "AIStimulus Structure"))
  (bind _pal (`self.Pal`))
  (`KismetSystemLibrary.PrintString` (`KismetSystemLibrary.GetDisplayName` Actor))
  (bind _targetactor (`self.TargetActor`)
    (:`then`
      (if (!= _targetactor Actor)
        (if (> (`self.GetDistanceTo` _pal (`self.TargetActor`)) (`self.GetDistanceTo` Actor _pal))
          (bind _output_get (set `self.TargetActor` Actor))
          (cast `/Game/Blueprint/Character/Player/BP_PlayerCharacter` _output_get
            (:`then`
              (`BaseAbilitySystemComponent.TryActivateAbilityByTag` (`BaseCharacter.BaseAbilitySystemComponent` (`self.Pal`)) (struct :`TagName` "Pal.Event.Encount") :!label _label))
            (:`CastFailed`
              _))
          (`BlackboardComponent.SetValueAsObject` (`AIBlueprintHelperLibrary.GetBlackboard` null) "TargetActor" _output_get))))
    (:`else`
      (set `self.TargetActor` Actor)
      (goto _label))))

(event `self.AIPerceptionComponent.OnTargetPerceptionForgotten`
  (params (Actor :type "Actor Object Reference"))
  (if (== Actor (`self.TargetActor`))
    (bind _output_get (set `self.TargetActor` null))
    (`BlackboardComponent.SetValueAsObject` (`AIBlueprintHelperLibrary.GetBlackboard` null) "TargetActor" _output_get)
    (`/Game/Blueprint/Character/Pal/BP_PalCharacterBase.SetState` (`self.Pal`) "NewEnumerator11")))

(fn `SetParentActor`
  (params (ParentActor :type "PlayerCharacter Object Reference"))
  (bind _output_get (set `self.ParentActor` ParentActor))
  (`BlackboardComponent.SetValueAsObject` (`AIBlueprintHelperLibrary.GetBlackboard` null) "ParentActor" _output_get))

(fn `UserConstructionScript`)