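; Laser beam skill actor for Pals, with a box hit volume and a tintable ray effect whose color is set at construction.
; On overlap it filters by AI team ID: players are hit unless the owning Pal is team 0, other Pals only if their team differs.
; Valid targets receive a HitReact gameplay event carrying damage calculated from skill damage and the owner's Attack.
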(event `self.Box.OnComponentBeginOverlap`
  (params (OverlappedComponent :type "PrimitiveComponent Object Reference") (OtherActor :type "Actor Object Reference") (OtherComp :type "PrimitiveComponent Object Reference") (OtherBodyIndex :type Integer) (bFromSweep :type Boolean) (SweepResult :type "HitResult Structure (by ref)"))
  (bind _asbase_character (cast `BaseCharacter` OtherActor))
  (bind _returnvalue (`BaseAIController.GetTeamId` (cast `/Game/Blueprint/Character/Pal/BP_BaseAIController` (`Pawn.GetController` (`self.Pal`)) :!pure true)))
  (set `self.Return Value Team ID` (break `GenericTeamId` _returnvalue))
  (cast `/Game/Blueprint/Character/Player/BP_PlayerCharacter` _asbase_character
    (:`then`
      (if (!= (`self.Return Value Team ID`) 0)
        (`AbilitySystemBlueprintLibrary.SendGameplayEventToActor` _asbase_character (struct :`TagName` "Shared.Event.HitReact") (make `GameplayEventData` (struct) null _asbase_character null null (struct) (struct) (struct) (`BaseFunctionLibrary.DamageCulculation` (`self.SkillDamage`) (`.Attack_64_6F50662A411440C79D9130B109D36331` (break `/Game/Blueprint/Component/Inventory/Struct/FPalProfileStruct` (`/Game/Blueprint/Character/Pal/BP_PalCharacterBase.Profile` (`self.Pal`)))))) :!label _label)))
    (:`CastFailed`
      (bind _asbp_pal_character_base (cast `/Game/Blueprint/Character/Pal/BP_PalCharacterBase` _asbase_character))
      (bind _returnvalue_2 (`BaseAIController.GetTeamId` (cast `/Game/Blueprint/Character/Pal/BP_BaseAIController` (`Pawn.GetController` _asbp_pal_character_base) :!pure true)))
      (if (!= (break `GenericTeamId` _returnvalue_2) (`self.Return Value Team ID`))
        (goto _label)))))

(fn `UserConstructionScript`
  (`FXSystemComponent.SetColorParameter` (`self.NS_Ray`) "Color" (`self.Color`)))