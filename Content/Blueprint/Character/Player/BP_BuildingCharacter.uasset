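; Player character for building and crafting, which creates the build menu widget and hands its follow camera to BPCBuildComponent.
; Input actions place builds or crafts through that component, with a continuous-build option that stays in build mode.
; Camera line traces delete BuildPart-tagged actors and send damage or press/release craft-interact messages.
; Key 3 runs a hold-progress delay loop that destroys the traced build if it reports unfinished.
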(event `self.ReceiveBeginPlay`
  (set `/Game/Blueprint/Component/Build/BPC_BuildComponent.Camera` (`self.FollowCamera`) (`self.BPC_BuildComponent`))
  (bind _returnvalue (`|CreateWidget` "/Game/Blueprint/Build/BuildMenu/WBP_BuildMenu.WBP_BuildMenu_C"))
  (set `self.BuildMenu` _returnvalue))

(event `DestroyComponent`
  (params (Component :type "ActorComponent Object Reference"))
  (`ActorComponent.K2_DestroyComponent` Component))

(event `EnhancedInput|/Game/Blueprint/Character/Player/Input/Actions/IA_PlaceBuild`
  (params (ActionValue :type Boolean) (ElapsedSeconds :type "Float (double-precision)") (TriggeredSeconds :type "Float (double-precision)") (InputAction :type "InputAction Object Reference" :default "/Game/Blueprint/Character/Player/Input/Actions/IA_PlaceBuild.IA_PlaceBuild"))
  (bind _bpc_buildcomponent (`self.BPC_BuildComponent`))
  (bind _bpc_buildcomponent_2 (`self.BPC_BuildComponent`))
  (bind _bpc_buildcomponent_3 (`self.BPC_BuildComponent`))
  (bind _bpc_buildcomponent_4 (`self.BPC_BuildComponent`))
  (:`Started`
    (`|ExecutionSequence`
      (:`then_0`
        (if (and (`/Game/Blueprint/Component/Build/BPC_BuildComponent.IsBuildMode` _bpc_buildcomponent) (`/Game/Blueprint/Component/Build/BPC_BuildComponent.CanBuild` _bpc_buildcomponent))
          (`/Game/Blueprint/Component/Build/BPC_BuildComponent.SpawnBuild` _bpc_buildcomponent_3)
          (`/Game/Blueprint/Component/Build/BPC_BuildComponent.StopBuildMode` _bpc_buildcomponent_3)))
      (:`then_1`
        (if (and (`/Game/Blueprint/Component/Build/BPC_BuildComponent.IsCraftMode` _bpc_buildcomponent_4) (`/Game/Blueprint/Component/Build/BPC_BuildComponent.CanCraft` _bpc_buildcomponent_4))
          (`/Game/Blueprint/Component/Build/BPC_BuildComponent.SpawnCraft` _bpc_buildcomponent_2)
          (`/Game/Blueprint/Component/Build/BPC_BuildComponent.StopCraftMode` _bpc_buildcomponent_2))))))

(event `EnhancedInput|/Game/Blueprint/Character/Player/Input/Actions/IA_ContinuousBuild`
  (params (ActionValue :type Boolean) (ElapsedSeconds :type "Float (double-precision)") (TriggeredSeconds :type "Float (double-precision)") (InputAction :type "InputAction Object Reference" :default "/Game/Blueprint/Character/Player/Input/Actions/IA_ContinuousBuild.IA_ContinuousBuild"))
  (bind _bpc_buildcomponent (`self.BPC_BuildComponent`))
  (:`Started`
    (if (and (`/Game/Blueprint/Component/Build/BPC_BuildComponent.IsBuildMode` _bpc_buildcomponent) (`/Game/Blueprint/Component/Build/BPC_BuildComponent.CanBuild` _bpc_buildcomponent))
      (`/Game/Blueprint/Component/Build/BPC_BuildComponent.SpawnBuild` (`self.BPC_BuildComponent`)))))

(event `EnhancedInput|/Game/Blueprint/Character/Player/Input/Actions/IA_Destroy`
  (params (ActionValue :type Boolean) (ElapsedSeconds :type "Float (double-precision)") (TriggeredSeconds :type "Float (double-precision)") (InputAction :type "InputAction Object Reference" :default "/Game/Blueprint/Character/Player/Input/Actions/IA_Destroy.IA_Destroy"))
  (bind _followcamera (`self.FollowCamera`))
  (bind _returnvalue (`SceneComponent.K2_GetComponentLocation` _followcamera))
  (bind _returnvalue_2 (`SceneComponent.GetForwardVector` _followcamera))
  (:`Started`
    (bind (_outhit _returnvalue_3) (`KismetSystemLibrary.LineTraceSingle` (+ _returnvalue (* _returnvalue_2 250.0)) (+ _returnvalue (* _returnvalue_2 900.0)) "TraceTypeQuery1"))
    (if _returnvalue_3
      (bind (_bblockinghit _binitialoverlap _time _distance _location _impactpoint _normal _impactnormal _physmat _hitactor) (`GameplayStatics.BreakHitResult` _outhit))
      (if (`self.ActorHasTag` _hitactor "BuildPart")
        (`self.K2_DestroyActor` _hitactor)))))

(event `Key|Three`
  (params (Key :type "Key Structure"))
  (:`Pressed`
    (bind _hitactor (`self.BuildTrace`))
    (if (`KismetSystemLibrary.DoesImplementInterface` _hitactor "/Game/Blueprint/Build/Building/BPI_BuildingInterface.BPI_BuildingInterface_C")
      (bind _isfinished (message `/Game/Blueprint/Build/Building/BPI_BuildingInterface.BuildFinished` _hitactor))
      (if (not _isfinished)
        (set `self.InProgress` true)
        (`self.ProgressAdd` :!label _label)
        (if (< (`self.ProgressValue`) 1.0)
          (`KismetSystemLibrary.Delay` 0.01)
          (goto _label)
          (else
            (set `self.InProgress` false)
            (set `self.ProgressValue` 0.0)
            (`self.K2_DestroyActor` _hitactor))))))
  (:`Released`
    (set `self.InProgress` false)
    (set `self.ProgressValue` 0.0)))

(event `ProgressAdd`
  (if (`self.InProgress`)
    (set `self.ProgressValue` (`KismetMathLibrary.FClamp` (+ (`self.ProgressValue`) 0.01)))))

(event `Key|Four`
  (params (Key :type "Key Structure"))
  (:`Pressed`
    (bind _hitactor (`self.BuildTrace`))
    (message `/Game/Blueprint/Build/Building/BPI_BuildingInterface.DealDamage` _hitactor 100.0)))

(event `EnhancedInput|/Game/Blueprint/Character/Player/Input/Actions/IA_Interact`
  (params (ActionValue :type "Vector2D Structure") (ElapsedSeconds :type "Float (double-precision)") (TriggeredSeconds :type "Float (double-precision)") (InputAction :type "InputAction Object Reference" :default "/Game/Blueprint/Character/Player/Input/Actions/IA_Interact.IA_Interact"))
  (bind _returnvalue (`GameplayStatics.GetPlayerCameraManager` 0))
  (bind _istriggered (`self.IsTriggered`))
  (bind _returnvalue_2 (`self.K2_GetActorLocation` _returnvalue))
  (:`Started`
    (set `self.IsTriggered` true)
    (bind (_outhit _returnvalue_3) (`KismetSystemLibrary.LineTraceSingle` _returnvalue_2 (+ _returnvalue_2 (* (`KismetMathLibrary.GetForwardVector` (`self.K2_GetActorRotation` _returnvalue)) 1000.0)) "TraceTypeQuery1" :!label _label_2))
    (if _returnvalue_3
      (`KismetSystemLibrary.PrintString` (`KismetStringLibrary.Conv_BoolToString` _istriggered))
      (message `/Game/Blueprint/Craft_Test/Crafting/BPI_CraftingInterface.InteractWithCraft` (`.HitActor` (`GameplayStatics.BreakHitResult` _outhit)) _istriggered)))
  (:`Completed`
    (set `self.IsTriggered` false)
    (goto _label_2)))

(fn `BuildFinished`
  (returns (IsFinished :type Boolean))
  (return false))

(fn `BuildTrace`
  (returns (HitActor :type "Actor Object Reference"))
  (bind _returnvalue (`GameplayStatics.GetPlayerCameraManager` 0))
  (bind _returnvalue_2 (`self.K2_GetActorLocation` _returnvalue))
  (bind (_outhit _returnvalue_3) (`KismetSystemLibrary.LineTraceSingle` _returnvalue_2 (+ _returnvalue_2 (* (`KismetMathLibrary.GetForwardVector` (`self.K2_GetActorRotation` _returnvalue)) 1000.0)) "TraceTypeQuery1"))
  (if _returnvalue_3
    _
    (else
      _))
  (return (`.HitActor` (`GameplayStatics.BreakHitResult` _outhit))))

(fn `CraftTrace`
  (returns (HitActor :type "Actor Object Reference"))
  (bind _returnvalue (`GameplayStatics.GetPlayerCameraManager` 0))
  (bind _returnvalue_2 (`self.K2_GetActorLocation` _returnvalue))
  (bind (_outhit _returnvalue_3) (`KismetSystemLibrary.LineTraceSingle` _returnvalue_2 (+ _returnvalue_2 (* (`KismetMathLibrary.GetForwardVector` (`self.K2_GetActorRotation` _returnvalue)) 1000.0)) "TraceTypeQuery1"))
  (if _returnvalue_3
    (return (`.HitActor` (`GameplayStatics.BreakHitResult` _outhit)))))

(fn `ReturnBoxes`
  (returns (Boxes :type "Array of BoxComponent Object Reference"))
  (return))

(fn `ReturnBuildID`
  (returns (BuildID :type Integer))
  (return 0))

(fn `ReturnCraftBoxes`
  (returns (Boxes :type "Array of BoxComponent Object Reference"))
  (return))

(fn `UserConstructionScript`)