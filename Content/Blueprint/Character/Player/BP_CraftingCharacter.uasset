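; Player character Blueprint that adds craft placement and world interaction through input, delegating craft logic to BPCCraftComponent, which receives the follow camera on BeginPlay.
; Craft input launches craft mode, keys 1 and 2 step the clamped craftable index and refresh the mesh, and place input spawns the craft when allowed, then exits the mode.
; Interact press and release both line-trace from the camera and send the hit actor InteractWithCraftMessage with the trigger state.
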(event `self.ReceiveBeginPlay`
  (set `/Game/Blueprint/Component/Craft_Test/BPC_CraftComponent.Camera` (`self.FollowCamera`) (`self.BPC_CraftComponent`)))

(event `EnhancedInput|/Game/Blueprint/Character/Player/Input/Actions/IA_Craft`
  (params (ActionValue :type Boolean) (ElapsedSeconds :type "Float (double-precision)") (TriggeredSeconds :type "Float (double-precision)") (InputAction :type "InputAction Object Reference" :default "/Game/Blueprint/Character/Player/Input/Actions/IA_Craft.IA_Craft"))
  (:`Started`
    (`/Game/Blueprint/Component/Craft_Test/BPC_CraftComponent.LaunchCraftMode` (`self.BPC_CraftComponent`))))

(event `DestroyComponent`
  (params (Component :type "ActorComponent Object Reference"))
  (`ActorComponent.K2_DestroyComponent` Component))

(event `Key|One`
  (params (Key :type "Key Structure"))
  (bind _bpc_craftcomponent (`self.BPC_CraftComponent`))
  (bind _bpc_craftcomponent_2 (`self.BPC_CraftComponent`))
  (:`Pressed`
    (if (`/Game/Blueprint/Component/Craft_Test/BPC_CraftComponent.IsCraftMode` _bpc_craftcomponent_2)
      (set `/Game/Blueprint/Component/Craft_Test/BPC_CraftComponent.CraftID` (`KismetMathLibrary.Clamp` (+ (`/Game/Blueprint/Component/Craft_Test/BPC_CraftComponent.CraftID` _bpc_craftcomponent_2) 1) 0 (- (`KismetArrayLibrary.Array_Length` (`/Game/Blueprint/Component/Craft_Test/BPC_CraftComponent.Craftable` _bpc_craftcomponent_2)) 1)) _bpc_craftcomponent)
      (`/Game/Blueprint/Component/Craft_Test/BPC_CraftComponent.ChangeMesh` _bpc_craftcomponent :!label _label))))

(event `Key|Two`
  (params (Key :type "Key Structure"))
  (bind _bpc_craftcomponent (`self.BPC_CraftComponent`))
  (:`Pressed`
    (if (`/Game/Blueprint/Component/Craft_Test/BPC_CraftComponent.IsCraftMode` _bpc_craftcomponent)
      (set `/Game/Blueprint/Component/Craft_Test/BPC_CraftComponent.CraftID` (`KismetMathLibrary.Clamp` (- (`/Game/Blueprint/Component/Craft_Test/BPC_CraftComponent.CraftID` _bpc_craftcomponent) 1) 0 (- (`KismetArrayLibrary.Array_Length` (`/Game/Blueprint/Component/Craft_Test/BPC_CraftComponent.Craftable` _bpc_craftcomponent)) 1)) (`self.BPC_CraftComponent`))
      (goto _label))))

(event `EnhancedInput|/Game/Blueprint/Character/Player/Input/Actions/IA_PlaceCraft`
  (params (ActionValue :type Boolean) (ElapsedSeconds :type "Float (double-precision)") (TriggeredSeconds :type "Float (double-precision)") (InputAction :type "InputAction Object Reference" :default "/Game/Blueprint/Character/Player/Input/Actions/IA_PlaceCraft.IA_PlaceCraft"))
  (bind _bpc_craftcomponent (`self.BPC_CraftComponent`))
  (bind _bpc_craftcomponent_2 (`self.BPC_CraftComponent`))
  (:`Started`
    (if (and (`/Game/Blueprint/Component/Craft_Test/BPC_CraftComponent.IsCraftMode` _bpc_craftcomponent) (`/Game/Blueprint/Component/Craft_Test/BPC_CraftComponent.CanCraft` _bpc_craftcomponent))
      (`/Game/Blueprint/Component/Craft_Test/BPC_CraftComponent.SpawnCraft` _bpc_craftcomponent_2)
      (`/Game/Blueprint/Component/Craft_Test/BPC_CraftComponent.StopCraftMode` _bpc_craftcomponent_2))))

(event `EnhancedInput|/Game/Blueprint/Character/Player/Input/Actions/IA_Interact`
  (params (ActionValue :type "Vector2D Structure") (ElapsedSeconds :type "Float (double-precision)") (TriggeredSeconds :type "Float (double-precision)") (InputAction :type "InputAction Object Reference" :default "/Game/Blueprint/Character/Player/Input/Actions/IA_Interact.IA_Interact"))
  (bind _returnvalue (`GameplayStatics.GetPlayerCameraManager` 0))
  (bind _returnvalue_2 (`self.K2_GetActorLocation` _returnvalue))
  (:`Started`
    (set `self.IsTriggered` true)
    (bind (_outhit _returnvalue_3) (`KismetSystemLibrary.LineTraceSingle` _returnvalue_2 (+ _returnvalue_2 (* (`KismetMathLibrary.GetForwardVector` (`self.K2_GetActorRotation` _returnvalue)) 1000.0)) "TraceTypeQuery1" :!label _label_2))
    (if _returnvalue_3
      (message `/Game/Blueprint/Craft_Test/Crafting/BPI_CraftingInterface.InteractWithCraft` (`.HitActor` (`GameplayStatics.BreakHitResult` _outhit)) (`self.IsTriggered`))))
  (:`Completed`
    (set `self.IsTriggered` false)
    (goto _label_2)))

(fn `ReturnBoxes`
  (returns (Boxes :type "Array of BoxComponent Object Reference"))
  (return))

(fn `ReturnCraftBoxes`
  (returns (Boxes :type "Array of BoxComponent Object Reference"))
  (return))

(fn `UserConstructionScript`)