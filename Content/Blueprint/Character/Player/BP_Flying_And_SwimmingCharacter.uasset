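; Player character Blueprint variant for flying and swimming, though only vertical flight control of the current Pal is wired.
; On BeginPlay it enables tick and puts its mesh into physics-simulated ragdoll.
; The up/down flight input feeds world-Z movement into the inventory manager's current Pal rather than this character.
; Move input and Tick are empty; horizontal Pal movement, fly mapping-context setup and ammo debug printing are left disconnected.
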(event `self.ReceiveBeginPlay`
  (bind _mesh (`self.Mesh`))
  (`parent.ReceiveBeginPlay`)
  (`self.SetActorTickEnabled` true)
  (`PrimitiveComponent.SetSimulatePhysics` _mesh true)
  (`PrimitiveComponent.SetCollisionProfileName` _mesh "Ragdoll" true))

(event `EnhancedInput|/Game/Blueprint/Character/Player/Input/Actions/IA_Move_Fly`
  (params (ActionValue :type "Vector2D Structure") (ElapsedSeconds :type "Float (double-precision)") (TriggeredSeconds :type "Float (double-precision)") (InputAction :type "InputAction Object Reference" :default "/Game/Blueprint/Character/Player/Input/Actions/IA_Move_Fly.IA_Move_Fly")))

(event `self.ReceiveTick`
  (params (DeltaSeconds :type "Float (single-precision)")))

(event `EnhancedInput|/Game/Blueprint/Character/Player/Input/Actions/IA_Flying_UpDawn`
  (params (ActionValue :type "Vector2D Structure") (ElapsedSeconds :type "Float (double-precision)") (TriggeredSeconds :type "Float (double-precision)") (InputAction :type "InputAction Object Reference" :default "/Game/Blueprint/Character/Player/Input/Actions/IA_Flying_UpDawn.IA_Flying_UpDawn"))
  (:`Triggered`
    (`self.AddMovementInput` (`/Game/Blueprint/Component/Inventory/PalInventorySystem.CurrentPal` (`/Game/Blueprint/Component/Inventory/InventoryManager.PalInventorySystem` (`self.InventoryManager`))) (0.0 0.0 1.0) ActionValue_X false)))

(fn `UserConstructionScript`
  (`parent.UserConstructionScript`))