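; Player controller that owns the local player's UI: the HUD and the display menu container.
; On BeginPlay it creates both widgets and adds them to the viewport, only on the local controller.
; SetCompass rotates the HUD compass by writing a scalar parameter on its dynamic material.
; UpdateWidget refreshes the HUD data, plus the player menu's data when that menu is the one held by the display menu.
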(event `self.ReceiveBeginPlay`
  (if (`self.IsLocalPlayerController`)
    (`|ExecutionSequence`
      (:`then_0`
        (bind _returnvalue (`|CreateWidget` "/Game/Blueprint/Component/Inventory/UI/Base/W_DisplayMenu.W_DisplayMenu_C"))
        (bind _output_get (set `self.PlayerMenu` _returnvalue))
        (`UserWidget.AddToViewport` _output_get 0))
      (:`then_1`
        (bind _returnvalue_2 (`|CreateWidget` "/Game/Blueprint/Component/Inventory/UI/W_HUD.W_HUD_C"))
        (bind _output_get_2 (set `self.HUD` _returnvalue_2))
        (`UserWidget.AddToViewport` _output_get_2 0)))))

(fn `SetCompass`
  (params (Compass :type "Float (double-precision)"))
  (bind _returnvalue (`Image.GetDynamicMaterial` (`/Game/Blueprint/Component/Inventory/UI/W_Compass.Compass` (`/Game/Blueprint/Component/Inventory/UI/W_HUD.W_Compass` (`self.HUD`)))))
  (`MaterialInstanceDynamic.SetScalarParameterValue` _returnvalue "CompassRotation" Compass))

(fn `UpdateWidget`
  (bind _menu (`/Game/Blueprint/Component/Inventory/UI/Base/W_DisplayMenu.Menu` (`self.PlayerMenu`)))
  (`/Game/Blueprint/Component/Inventory/UI/W_HUD.SetData` (`self.HUD`))
  (`/Engine/EditorBlueprintResources/StandardMacros.IsValid` _menu
    (:`Is Valid`
      (bind _asw_player_menu (cast `/Game/Blueprint/Component/Inventory/UI/W_PlayerMenu` _menu))
      (`/Game/Blueprint/Component/Inventory/UI/W_PlayerMenu.SetData` _asw_player_menu))))

(fn `UserConstructionScript`)