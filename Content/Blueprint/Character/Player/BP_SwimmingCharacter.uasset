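; Player character Blueprint that sets Head and Hair equipment meshes to follow the main mesh's pose, with prototype swimming logic left unwired.
; The construction script assigns the leader pose component.
; Swimming compares depth below WaterZ to capsule half-height, using paired DoOnce gates to toggle Swimming/Walking movement and the physics volume's water flag.
; That function returns on its first sequence pin, and its call and the water enter/exit nodes never run.
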(event `self.ReceiveBeginPlay`)

(event `self.ReceiveTick`
  (params (DeltaSeconds :type "Float (single-precision)")))

(fn `UserConstructionScript`
  (`SkinnedMeshComponent.SetLeaderPoseComponent` (`BlueprintMapLibrary.Map_Find` (`self.CharacterEquipmentMap`) "Head") (`self.Mesh`) false false)
  (`SkinnedMeshComponent.SetLeaderPoseComponent` (`BlueprintMapLibrary.Map_Find` (`self.CharacterEquipmentMap`) "Hair") (`self.Mesh`) false false))