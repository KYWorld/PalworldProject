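; BP_Flying is a player character Blueprint that adds a toggleable flying mode.
; On BeginPlay it adds the IMC_Flying Enhanced Input context, whose up/down action moves the character vertically while flying.
; A hard-coded Space Bar double-tap, tracked by a counter reset after a retriggerable delay, flip-flops movement between Flying and Falling.
; Landing restores Walking; alternative jump and delayed-walk logic is left unconnected.
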(event `self.ReceiveBeginPlay`
  (`parent.ReceiveBeginPlay`)
  (`EnhancedInputSubsystemInterface.AddMappingContext` (pcsubsystem `EnhancedInputLocalPlayerSubsystem` (`GameplayStatics.GetPlayerController` 0)) "/Game/Blueprint/Character/Player/Input/IMC_Flying.IMC_Flying" 1 (struct)))

(event `EnhancedInput|/Game/Blueprint/Character/Player/Input/Actions/IA_Flying_UpDawn`
  (params (ActionValue :type "Vector2D Structure") (ElapsedSeconds :type "Float (double-precision)") (TriggeredSeconds :type "Float (double-precision)") (InputAction :type "InputAction Object Reference" :default "/Game/Blueprint/Character/Player/Input/Actions/IA_Flying_UpDawn.IA_Flying_UpDawn"))
  (:`Triggered`
    (if (`NavMovementComponent.IsFlying` (`self.CharacterMovement`))
      (`self.AddMovementInput` (0.0 0.0 1.0) ActionValue_X))))

(event `Key|SpaceBar`
  (params (Key :type "Key Structure"))
  (bind _charactermovement (`self.CharacterMovement`))
  (:`Pressed`
    (bind _result (`/Engine/EditorBlueprintResources/StandardMacros.IncrementInt` (`self.Combo`))
      (:`  `
        (if (== _result 2)
          (`/Engine/EditorBlueprintResources/StandardMacros.FlipFlop`
            (:`A`
              (`CharacterMovementComponent.SetMovementMode` _charactermovement "MOVE_Flying" 0))
            (:`B`
              (`CharacterMovementComponent.SetMovementMode` _charactermovement "MOVE_Falling" 0)))
          (else
            (`KismetSystemLibrary.RetriggerableDelay` 0.5)
            (set `self.Combo` 0)))))))

(event `self.OnLanded`
  (params (Hit :type "HitResult Structure (by ref)"))
  (`CharacterMovementComponent.SetMovementMode` (`self.CharacterMovement`) "MOVE_Walking" 0))

(fn `UserConstructionScript`
  (`parent.UserConstructionScript`))