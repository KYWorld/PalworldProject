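; Player character component that switches movement between Swimming and Walking based on how far the character sinks below the water height recorded on entry.
; While in water, the Tick-driven Swimming macro compares depth to capsule half-height, using cross-resetting DoOnce gates to fire each switch once.
; Switches toggle the physics volume's WaterVolume flag; starting to swim also cancels gliding and zeroes velocity.
; An older timer chain (Z, Up, IsGround) remains but is never started.
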(event `self.ReceiveBeginPlay`
  (bind _asbp_player_character (cast `/Game/Blueprint/Character/Player/BP_PlayerCharacter` (`self.GetOwner`)))
  (bind _output_get (set `self.As BP Player Character` _asbp_player_character))
  (set `self.Character Movement_0` (`Character.CharacterMovement` _output_get)))

(event `/Game/Blueprint/Character/Player/Swimming/BPI_SwimmingInterface.F_EnterWater`
  (bind (_returnvalue_x _returnvalue_y _returnvalue_z) (`KismetMathLibrary.BreakVector` (`Actor.K2_GetActorLocation` (`self.As BP Player Character`))))
  (set `self.InWater` true)
  (set `self.WaterZ` _returnvalue_z))

(event `Z`
  (bind _character_movement_0 (`self.Character Movement_0`))
  (bind (_returnvalue_x _returnvalue_y _returnvalue_z) (`KismetMathLibrary.BreakVector` (`Actor.K2_GetActorLocation` (`self.As BP Player Character`))))
  (if (> (- (`self.WaterZ`) _returnvalue_z) (- (`CapsuleComponent.CapsuleHalfHeight` (`Character.CapsuleComponent` (`self.As BP Player Character`))) 50.0))
    (set `PhysicsVolume.bWaterVolume` true (`MovementComponent.GetPhysicsVolume` _character_movement_0))
    (set `CharacterMovementComponent.Buoyancy` 1.0 _character_movement_0)
    (`CharacterMovementComponent.SetMovementMode` _character_movement_0 "MOVE_Swimming" 0)
    (`KismetSystemLibrary.K2_ClearAndInvalidateTimerHandle` (`self.Z_TimerHandle`))
    (bind _returnvalue (`KismetSystemLibrary.K2_SetTimerDelegate` (delegate `Up`) 0.01 true))
    (set `self.Up_TimerHandle` _returnvalue)))

(event `Up`
  (bind _as_bp_player_character (`self.As BP Player Character`))
  (bind (_returnvalue_x _returnvalue_y) (`KismetMathLibrary.BreakVector` (`Actor.K2_GetActorLocation` _as_bp_player_character)))
  (`Actor.K2_SetActorLocation` _as_bp_player_character (`KismetMathLibrary.MakeVector` _returnvalue_x _returnvalue_y (- (`self.WaterZ`) 100.0)) false false)
  (`KismetSystemLibrary.Delay` 3.0)
  (`KismetSystemLibrary.K2_ClearAndInvalidateTimerHandle` (`self.Up_TimerHandle`))
  (bind _returnvalue (`KismetSystemLibrary.K2_SetTimerDelegate` (delegate `IsGround`) 0.01 true))
  (set `self.Ground_TimerHandle` _returnvalue))

(event `IsGround`
  (bind _character_movement_0 (`self.Character Movement_0`))
  (bind (_returnvalue_x _returnvalue_y _returnvalue_z) (`KismetMathLibrary.BreakVector` (`Actor.K2_GetActorLocation` (`self.As BP Player Character`))))
  (if (not (> (- (`self.WaterZ`) _returnvalue_z) (`CapsuleComponent.CapsuleHalfHeight` (`Character.CapsuleComponent` (`self.As BP Player Character`)))))
    (`KismetSystemLibrary.K2_ClearAndInvalidateTimerHandle` (`self.Ground_TimerHandle`))
    (set `PhysicsVolume.bWaterVolume` false (`MovementComponent.GetPhysicsVolume` _character_movement_0))
    (`CharacterMovementComponent.SetMovementMode` _character_movement_0 "MOVE_Walking" 0)))

(event `/Game/Blueprint/Character/Player/Swimming/BPI_SwimmingInterface.F_ExitWater`
  (set `self.InWater` false))

(event `self.ReceiveTick`
  (params (DeltaSeconds :type "Float (single-precision)"))
  (bind _waterz (`self.WaterZ`))
  (bind _character_movement_0 (`self.Character Movement_0`))
  (bind _character_movement_0_2 (`self.Character Movement_0`))
  (bind (_returnvalue_x _returnvalue_y _returnvalue_z) (`KismetMathLibrary.BreakVector` (`Actor.K2_GetActorLocation` (`self.As BP Player Character`))))
  (bind _capsulehalfheight (`CapsuleComponent.CapsuleHalfHeight` (`Character.CapsuleComponent` (`self.As BP Player Character`))))
  (`|ExecutionSequence`
    (:`then_1`
      (if (`self.InWater`)
        (if (> (- _waterz _returnvalue_z) _capsulehalfheight)
          (`/Engine/EditorBlueprintResources/StandardMacros.DoOnce` false :!label _label
            (:`Completed`
              (`BaseAbilitySystemComponent.TryCancelAbilityByTag` (`BaseCharacter.BaseAbilitySystemComponent` (`self.As BP Player Character`)) (struct :`TagName` "InputTag.Gliding"))
              (set `PhysicsVolume.bWaterVolume` true (`MovementComponent.GetPhysicsVolume` _character_movement_0))
              (`CharacterMovementComponent.SetMovementMode` _character_movement_0 "MOVE_Swimming" 0)
              (set `MovementComponent.Velocity` (0.0 0.0 0.0) _character_movement_0)
              (goto _label_2 :!via `Reset`)))
          (elif (< (- _waterz _returnvalue_z) (/ _capsulehalfheight 1.0))
            (`/Engine/EditorBlueprintResources/StandardMacros.DoOnce` false :!label _label_2
              (:`Completed`
                (set `PhysicsVolume.bWaterVolume` false (`MovementComponent.GetPhysicsVolume` _character_movement_0_2))
                (`CharacterMovementComponent.SetMovementMode` _character_movement_0_2 "MOVE_Walking" 0)
                (goto _label :!via `Reset`)))))))))

(fn `GravityScale`
  (params (NewParam :type "Float (double-precision)"))
  (set `CharacterMovementComponent.GravityScale` NewParam (`Character.CharacterMovement` (`self.As BP Player Character`))))

(fn `NewFunction`
  (bind _as_bp_player_character (`self.As BP Player Character`))
  (bind _waterz (`self.WaterZ`))
  (bind (_returnvalue_x _returnvalue_y) (`KismetMathLibrary.BreakVector` (`Actor.K2_GetActorLocation` _as_bp_player_character)))
  (`KismetSystemLibrary.PrintString` (`KismetStringLibrary.Conv_DoubleToString` (- _waterz 6.0)))
  (`Actor.K2_SetActorLocation` _as_bp_player_character (`KismetMathLibrary.MakeVector` _returnvalue_x _returnvalue_y _waterz) false false))