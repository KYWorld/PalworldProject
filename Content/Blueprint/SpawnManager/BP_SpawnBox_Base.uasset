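; Base spawn volume that keeps a population of Pals inside its box, up to a maximum count.
; A looping timer prunes invalid Pals from the tracked array, then spawns one if below the limit.
; Each spawn picks a random data table row for class and stats, with randomized gender and weighted-random Weight.
; Locations come from navmesh queries within the box's bounding-sphere radius, retried until one succeeds.
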(event `self.ReceiveBeginPlay`
  (bind _returnvalue (`KismetSystemLibrary.K2_SetTimerDelegate` (delegate `Spawn`) (`self.SpawnRate`) true))
  (set `self.Handle` _returnvalue))

(event `Spawn`
  (`self.IsValidPalArray`)
  (if (< (`self.SpawnCount`) (`self.MaxSpawnCount`))
    (bind _location (`self.GetRandomLocation`))
    (`self.SpawnPal` _location)))

(fn `GetRandomLocation`
  (returns (Location :type "Vector Structure"))
  (bind (_origin _boxextent _sphereradius) (`KismetSystemLibrary.GetComponentBounds` (`self.Box`)))
  (bind (_randomlocation _returnvalue) (`NavigationSystemV1.K2_GetRandomLocationInNavigableRadius` _origin _sphereradius null null :!label _label))
  (if _returnvalue
    (return _randomlocation)
    (else
      (goto _label))))

(fn `IsValidPalArray`
  (locals (TempArray :type "Array of /Game/Blueprint/Character/Pal/BP_PalCharacterBase Object Reference"))
  (bind _palarray (`self.PalArray`))
  (bind (_arrayindex _arrayelement) (`/Engine/EditorBlueprintResources/StandardMacros.ReverseForEachLoop` _palarray)
    (:`LoopBody`
      (`/Engine/EditorBlueprintResources/StandardMacros.IsValid` _arrayelement
        (:`Is Not Valid`
          (`KismetArrayLibrary.Array_Remove` _palarray _arrayindex))))
    (:`Completed`
      (set `self.SpawnCount` (`KismetArrayLibrary.Array_Length` (`self.PalArray`))))))

(fn `SetProfile`
  (params (PalStruct :type "/Game/Blueprint/Component/Inventory/Struct/FPalStruct Structure"))
  (returns (PalProfile :type "/Game/Blueprint/Component/Inventory/Struct/FPalProfileStruct Structure"))
  (bind (_name _description _thumbnail _palclass _attack _defence _workspeed _maxenergy _element _maxhp) (break `/Game/Blueprint/Component/Inventory/Struct/FPalStruct` PalStruct))
  (return (make `/Game/Blueprint/Component/Inventory/Struct/FPalProfileStruct` 1 (`KismetArrayLibrary.Array_Random` (`|MakeArray` "NewEnumerator0" "NewEnumerator1" :!type "/Game/Blueprint/Enum/EGender Enum")) false (`KismetArrayLibrary.Array_Random` (`|MakeArray` "NewEnumerator11" "NewEnumerator12" "NewEnumerator12" "NewEnumerator13" "NewEnumerator13" "NewEnumerator14" :!type "/Game/Blueprint/Enum/EPalWeight Enum")) _attack _defence _workspeed _maxenergy (make `GenericTeamId` 1) false _maxhp 0.0 _maxhp 100.0 _maxenergy)))

(fn `SpawnPal`
  (params (Location :type "Vector Structure"))
  (bind _returnvalue (`|GetDataTableRow` "/Game/Blueprint/Component/Inventory/DataTable/DT_PalData.DT_PalData" (`.RowName` (break `DataTableRowHandle` (`KismetArrayLibrary.Array_Random` (`self.SpawnData`)))))
    (:`then`
      (bind _returnvalue_2 (`|SpawnActorFromClass` (`.PalClass_46_862F52B649AEE6ABB7A0A2A921B1159B` (break `/Game/Blueprint/Component/Inventory/Struct/FPalStruct` _returnvalue)) (`KismetMathLibrary.MakeTransform` Location) "Undefined" "MultiplyWithRoot" null (`self.SetProfile` _returnvalue) -1 null))
      (`KismetArrayLibrary.Array_Add` (`self.PalArray`) _returnvalue_2)
      (`/Engine/EditorBlueprintResources/StandardMacros.IncrementInt` (`self.SpawnCount`)))))

(fn `UserConstructionScript`)