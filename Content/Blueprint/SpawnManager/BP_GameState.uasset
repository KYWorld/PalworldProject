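; BP_GameState drives a looping day cycle by rotating the level's directional light.
; BeginPlay caches the first DirectionalLight found, and Tick advances TimeOfDay by delta time scaled by DaySpeed, applying it as the light's pitch.
; Past a threshold, intensity drops a fixed step per tick down to zero, making the fade frame-rate dependent.
; At the cycle's end, time wraps back and full intensity returns instantly.
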(event `self.ReceiveBeginPlay`
  (bind _outactors (`GameplayStatics.GetAllActorsOfClass` "/Script/Engine.DirectionalLight"))
  (bind _output (`|GetArrayItem` _outactors))
  (`/Engine/EditorBlueprintResources/StandardMacros.IsValid` _output
    (:`Is Valid`
      (set `self.DirectionalLight` _output))))

(event `self.ReceiveTick`
  (params (DeltaSeconds :type "Float (single-precision)"))
  (`self.UpdateTime` DeltaSeconds))

(fn `UpdateTime`
  (params (DeltaSecond :type "Float (double-precision)"))
  (bind _lightcomponent (`Light.LightComponent` (`self.DirectionalLight`)))
  (bind _output_get (set `self.TimeOfDay` (+ (`self.TimeOfDay`) (* DeltaSecond (`self.DaySpeed`)))))
  (if (> _output_get 450.0)
    (set `self.TimeOfDay` 170.0)
    (`LightComponent.SetIntensity` (`Light.LightComponent` (`self.DirectionalLight`)) 18.0)
    (elif (> _output_get 360.0)
      (`LightComponent.SetIntensity` _lightcomponent (`KismetMathLibrary.FClamp` (- (`LightComponentBase.Intensity` _lightcomponent) 1.0) 0.0 18.0))))
  (`self.K2_SetActorRotation` (`self.DirectionalLight`) (`KismetMathLibrary.MakeRotator` 0.0 (`self.TimeOfDay`)) false))

(fn `UserConstructionScript`)