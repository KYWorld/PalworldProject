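; Base component for mineable foliage that drops resource items when a component owned by the player character overlaps it.
; On BeginPlay it binds its own begin-overlap event, which filters for BP_PlayerCharacter as owner.
; It then spawns an emitter and a random DropItem class at the overlapping component's location, enabling mesh physics on ResourceItemBase drops.
; The graph does not remove or alter the foliage itself.
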(event `self.ReceiveBeginPlay`
  (add `self.OnComponentBeginOverlap` (delegate `BeginOverlap`)))

(event `BeginOverlap` :!signature `self.OnComponentBeginOverlap`
  (params (OverlappedComponent :type "PrimitiveComponent Object Reference") (OtherActor :type "Actor Object Reference") (OtherComp :type "PrimitiveComponent Object Reference") (OtherBodyIndex :type Integer) (bFromSweep :type Boolean) (SweepResult :type "HitResult Structure (by ref)"))
  (bind _returnvalue (`self.K2_GetComponentLocation` OtherComp))
  (cast `/Game/Blueprint/Character/Player/BP_PlayerCharacter` (`self.GetOwner` OtherComp))
  (`GameplayStatics.SpawnEmitterAtLocation` (`self.Emitter Template`) _returnvalue (`self.K2_GetComponentRotation` OtherComp))
  (bind _returnvalue_2 (`|SpawnActorFromClass` (`KismetArrayLibrary.Array_Random` (`self.DropItem`)) (`KismetMathLibrary.MakeTransform` _returnvalue) "Undefined" "MultiplyWithRoot" null null))
  (bind _asresource_item_base (cast `ResourceItemBase` _returnvalue_2))
  (`self.SetSimulatePhysics` (`ResourceItemBase.ResourceItemMesh` _asresource_item_base) true))