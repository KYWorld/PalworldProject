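; BPC_InteractableFoliage_Base is a component that makes its owner, apparently interactable foliage, carry pickup item data.
; On BeginPlay it adds an ItemDataComponent to the owner and copies in the item ID and quantity.
; LookAt looks up the item row but returns an empty string, with its "Pick up" widget message disconnected.
; SetVisibilityWidget applies a material choice involving an outline, prints a debug string and leaves its hide logic unwired.
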(event `self.ReceiveBeginPlay`
  (bind _returnvalue (`|AddComponentByClass` (`self.GetOwner`) "/Game/Blueprint/Component/Inventory/ItemDataComponent.ItemDataComponent_C"))
  (set `/Game/Blueprint/Component/Inventory/ItemDataComponent.ItemID` (`self.Data`) _returnvalue)
  (set `/Game/Blueprint/Component/Inventory/ItemDataComponent.Quantity` (`self.Quantity`) _returnvalue))

(fn `LookAt`
  (returns (Message :type Text))
  (bind (_data_datatable _data_rowname) (break `DataTableRowHandle` (`self.Data`)))
  (bind _returnvalue (`|GetDataTableRow` "/Game/Blueprint/Component/Inventory/DataTable/DT_ItemData.DT_ItemData" _data_rowname)
    (:`then`
      (return ""))))

(fn `Set Visibility Widget`
  (params (Result :type Boolean))
  (returns (NewParam :type Boolean))
  (`StaticMesh.AddMaterial` (`self.StaticMesh`) (select `bool` Result :`false` "/Game/Blueprint/Material/M_Outline.M_Outline" :!type "MaterialInterface Object Reference"))
  (`KismetSystemLibrary.PrintString` "Hello")
  (return false))