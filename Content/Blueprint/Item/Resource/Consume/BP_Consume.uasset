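; BP_Consume is a consumable resource item actor that presents a pickup prompt when looked at.
; LookAt finds the item's data table row through its ItemDataComponent and shows "Pick up" with the item name in the W_DisplayInfo widget.
; SetVisibilityWidget toggles that widget together with an outline overlay material on the mesh, with a true input hiding both.
; The event graph is empty, and the pickup itself is not implemented here.
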(fn `LookAt`
  (returns (Message :type Text))
  (bind (_itemid_datatable _itemid_rowname) (break `DataTableRowHandle` (`/Game/Blueprint/Component/Inventory/ItemDataComponent.ItemID` (`self.ItemDataComponent`))))
  (bind _returnvalue (`|GetDataTableRow` _itemid_datatable _itemid_rowname)
    (:`then`
      (bind _asw_display_info (cast `/Game/Blueprint/Component/Inventory/UI/Base/W_DisplayInfo` (`WidgetComponent.GetWidget` (`self.Display Widget`))))
      (`/Game/Blueprint/Component/Inventory/UI/Base/W_DisplayInfo.ShowMessage` _asw_display_info (`|FormatText` "Pick up {Item}" (`.Name_2_26DE416D4415FAF52FE0AE8026C68146` (break `/Game/Blueprint/Component/Inventory/Struct/FItemStruct` _returnvalue))))
      (return ""))))

(fn `Set Visibility Widget`
  (params (Result :type Boolean))
  (returns (NewParam :type Boolean))
  (`MeshComponent.SetOverlayMaterial` (`self.ResourceItemMesh`) (select `bool` Result :`false` "/Game/Blueprint/Material/M_Outline.M_Outline" :!type "MaterialInterface Object Reference"))
  (`SceneComponent.SetHiddenInGame` (`self.Display Widget`) Result false)
  (return false))

(fn `UserConstructionScript`)