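; BP_PalSphere is the capture sphere item that catches a Pal on mesh overlap.
; On overlap it deactivates the Pal, stops its own physics and collision, then a timeline moves and scales up the sphere from the Pal to a random point ahead of player 0.
; When the sphere's montage completes, it sets the Pal's team ID to 0, sends it to the player's PalInventorySystem and destroys itself, with no success roll.
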(event `self.EquipmentItemMesh.OnComponentBeginOverlap`
  (params (OverlappedComponent :type "PrimitiveComponent Object Reference") (OtherActor :type "Actor Object Reference") (OtherComp :type "PrimitiveComponent Object Reference") (OtherBodyIndex :type Integer) (bFromSweep :type Boolean) (SweepResult :type "HitResult Structure (by ref)"))
  (bind _pal (`self.Pal`))
  (bind _asbp_pal_character_base (cast `/Game/Blueprint/Character/Pal/BP_PalCharacterBase` OtherActor))
  (bind _output_get (set `self.Pal` _asbp_pal_character_base))
  (`BaseCharacter.SetActivate` _output_get false)
  (`PrimitiveComponent.SetSimulatePhysics` (`self.EquipmentItemMesh`) false)
  (bind _asbp_player_character (cast `/Game/Blueprint/Character/Player/BP_PlayerCharacter` (`GameplayStatics.GetPlayerCharacter` 0)))
  (set `self.Player` _asbp_player_character)
  (set `self.EndLocation` (+ (`self.K2_GetActorLocation` (`self.Player`)) (* (`self.GetActorForwardVector` (`self.Player`)) 300.0) (* (`self.GetActorRightVector` (`self.Player`)) (`KismetMathLibrary.RandomFloatInRange` -200.0 200.0)) (* (`self.GetActorUpVector` (`self.Player`)) (`KismetMathLibrary.RandomFloatInRange` 100.0 250.0))))
  (set `self.StartLocation` (`self.K2_GetActorLocation` (`self.Pal`)))
  (`PrimitiveComponent.SetCollisionEnabled` (`self.EquipmentItemMesh`) "NoCollision")
  (bind (_direction _time) (`Timeline|MoveToCharacter` :!via `PlayFromStart`)
    (:`Update`
      (`self.K2_SetActorTransform` (`KismetMathLibrary.MakeTransform` (`KismetMathLibrary.VLerp` (`self.StartLocation`) (`self.EndLocation`) _time) (struct) (`KismetMathLibrary.VLerp` (0.01 0.01 0.01) (0.05 0.05 0.05) _time))))
    (:`Finished`
      (`|PlayMontage` (`self.EquipmentItemMesh`) "/Game/PalworldAsset/Weapons/SK_Weapon_PalSphere_001/Animation/SK_Weapon_PalSphere_001_Montage.SK_Weapon_PalSphere_001_Montage"
        (:`OnCompleted`
          ;[1 1 1] 잡았다면
          (bind _structout (setmembers `/Game/Blueprint/Component/Inventory/Struct/FPalProfileStruct` :`StructRef` (`/Game/Blueprint/Character/Pal/BP_PalCharacterBase.Profile` _pal) :`TeamID` (make `GenericTeamId` 0)))
          (set `/Game/Blueprint/Character/Pal/BP_PalCharacterBase.Profile` _structout _pal)
          (`/Game/Blueprint/Component/Inventory/InventorySystem.Server_Interact` (`/Game/Blueprint/Component/Inventory/InventoryManager.PalInventorySystem` (`/Game/Blueprint/Character/Player/BP_PlayerCharacter.InventoryManager` (`self.Player`))) (`self.Pal`))
          (`self.K2_DestroyActor`))))))

(fn `UserConstructionScript`
  (`parent.UserConstructionScript`))