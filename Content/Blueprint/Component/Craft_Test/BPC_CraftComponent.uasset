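; Build-mode component for BP_CraftingCharacter that previews and spawns placeable pieces loaded from DT_Crafting.
; While craft mode is on, CraftCycle re-runs on a short delay, camera-tracing to position a collisionless ghost mesh that input can rotate.
; The ghost snaps to craft boxes reported by the hit actor, then a bounds-sized box trace tints it green or red and sets CanCraft.
; SpawnCraft spawns the selected actor, passing mesh and cost.
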(event `self.ReceiveBeginPlay`
  (bind _asbp_crafting_character (cast `/Game/Blueprint/Character/Player/BP_CraftingCharacter` (`self.GetOwner`)))
  (set `self.Player` _asbp_crafting_character)
  (bind _outrownames (`DataTableFunctionLibrary.GetDataTableRowNames` "/Game/Blueprint/Craft_Test/Crafting/DT_Crafting.DT_Crafting"))
  (for _array_element _outrownames
    (bind _returnvalue (`|GetDataTableRow` "/Game/Blueprint/Craft_Test/Crafting/DT_Crafting.DT_Crafting" _array_element)
      (:`then`
        (`KismetArrayLibrary.Array_Add` (`self.Craftable`) _returnvalue)))))

(event `DestroyComponent`
  (params (Component :type "ActorComponent Object Reference"))
  (`self.K2_DestroyComponent` Component))

(event `CraftDelay`
  (bind _craftghost (`self.CraftGhost`))
  (if (`self.IsCraftMode`)
    (`KismetSystemLibrary.Delay` 0.01)
    (`self.CraftCycle`)
    (else
      (set `self.IsCraftMode` false :!label _label)
      (set `self.CanCraft` false)
      (`/Engine/EditorBlueprintResources/StandardMacros.IsValid` _craftghost
        (:`Is Valid`
          (`/Game/Blueprint/Character/Player/BP_CraftingCharacter.DestroyComponent` (`self.Player`) _craftghost))))))

(event `StopCraftMode`
  (goto _label))

(event `LaunchCraftMode`
  (if (`self.IsCraftMode`)
    (`self.StopCraftMode`)
    (else
      (set `self.IsCraftMode` true)
      (`self.CraftCycle`))))

(event `EnhancedInput|/Game/Blueprint/Character/Player/Input/Actions/IA_RotateMesh`
  (params (ActionValue :type Boolean) (ElapsedSeconds :type "Float (double-precision)") (TriggeredSeconds :type "Float (double-precision)") (InputAction :type "InputAction Object Reference" :default "/Game/Blueprint/Character/Player/Input/Actions/IA_RotateMesh.IA_RotateMesh"))
  (bind (_crafttransform_location _crafttransform_rotation) (`KismetMathLibrary.BreakTransform` (`self.CraftTransform`)))
  (:`Started`
    (set `self.CraftRotation` (`KismetMathLibrary.ComposeRotators` _crafttransform_rotation (struct :`Yaw` 5.0)))))

(event `EnhancedInput|/Game/Blueprint/Character/Player/Input/Actions/IA_OppositeRotateMesh`
  (params (ActionValue :type Boolean) (ElapsedSeconds :type "Float (double-precision)") (TriggeredSeconds :type "Float (double-precision)") (InputAction :type "InputAction Object Reference" :default "/Game/Blueprint/Character/Player/Input/Actions/IA_OppositeRotateMesh.IA_OppositeRotateMesh"))
  (bind (_crafttransform_location _crafttransform_rotation) (`KismetMathLibrary.BreakTransform` (`self.CraftTransform`)))
  (:`Started`
    (set `self.CraftRotation` (`KismetMathLibrary.ComposeRotators` _crafttransform_rotation (struct :`Yaw` -5.0)))))

(fn `ChangeMesh`
  (bind (_output_name _output_mesh) (break `/Game/Blueprint/Craft_Test/Crafting/ST_Crafting` (`|GetArrayItem` (`self.Craftable`) (`self.CraftID`))))
  (`StaticMeshComponent.SetStaticMesh` (`self.CraftGhost`) _output_mesh))

(fn `CheckForOverlap`
  (returns (Hit :type Boolean))
  (bind (_origin _boxextent) (`KismetSystemLibrary.GetComponentBounds` (`self.CraftGhost`)))
  (bind (_outhit _returnvalue) (`KismetSystemLibrary.BoxTraceSingle` :`Start` _origin :`End` _origin :`HalfSize` (/ _boxextent 1.2) :`TraceChannel` "TraceTypeQuery1" :`DrawDebugType` "ForOneFrame"))
  (return _returnvalue))

(fn `CraftCycle`
  (bind _camera (`self.Camera`))
  (bind _craftghost (`self.CraftGhost`))
  (bind _craftrotation (`self.CraftRotation`))
  (bind _returnvalue (`SceneComponent.K2_GetComponentLocation` _camera))
  (bind _returnvalue_2 (`SceneComponent.GetForwardVector` _camera))
  (bind (_output_name _output_mesh _output_tracechannel) (break `/Game/Blueprint/Craft_Test/Crafting/ST_Crafting` (`|GetArrayItem` (`self.Craftable`) (`self.CraftID`))))
  (bind (_outhit _returnvalue_3) (`KismetSystemLibrary.LineTraceSingle` (+ _returnvalue (* _returnvalue_2 250.0)) (+ _returnvalue (* _returnvalue_2 900.0)) _output_tracechannel))
  (if _returnvalue_3
    (bind (_bblockinghit _binitialoverlap _time _distance _location _impactpoint _normal _impactnormal _physmat _hitactor _hitcomponent _hitbonename _bonename _hititem _elementindex _faceindex _tracestart _traceend) (`GameplayStatics.BreakHitResult` _outhit))
    (set `self.CraftTransform` (`KismetMathLibrary.MakeTransform` _impactpoint _craftrotation))
    (set `self.Hit Actor` _hitactor)
    (set `self.Hit Component` _hitcomponent)
    (`/Engine/EditorBlueprintResources/StandardMacros.IsValid` _craftghost
      (:`Is Valid`
        (bind (_found _transform) (`self.DetectCraftBoxes`))
        (if _found
          (set `self.CraftTransform` _transform))
        (bind _hit (`self.CheckForOverlap`))
        (if _hit
          (`self.GiveCraftColor` false)
          (else
            (`self.GiveCraftColor` true)))
        (`self.CraftDelay`))
      (:`Is Not Valid`
        (`self.SpawnCraftGhost` :!label _label)
        (`self.CraftDelay` :!label _label_2)))
    (else
      (set `self.CraftTransform` (`KismetMathLibrary.MakeTransform` _traceend _craftrotation))
      (`/Engine/EditorBlueprintResources/StandardMacros.IsValid` _craftghost
        (:`Is Valid`
          (`self.GiveCraftColor` false)
          (goto _label_2))
        (:`Is Not Valid`
          (goto _label))))))

(fn `DetectCraftBoxes`
  (returns (Found :type Boolean) (Transform :type "Transform Structure"))
  (locals (LocalFound :type Boolean))
  (bind _boxes (message `/Game/Blueprint/Craft_Test/Crafting/BPI_CraftingInterface.ReturnCraftBoxes` (`self.Hit Actor`)))
  (for _array_element _boxes
    (if (== _array_element (`self.Hit Component`))
      (set `local.LocalFound` true)
      (break)))
  (return (`local.LocalFound`) (`SceneComponent.K2_GetComponentToWorld` (`self.Hit Component`))))

(fn `GiveCraftColor`
  (params (IsGreen :type Boolean))
  (bind _craftghost (`self.CraftGhost`))
  (set `self.CanCraft` IsGreen)
  (for _index (range (`PrimitiveComponent.GetNumMaterials` (`self.CraftGhost`)))
    (if IsGreen
      (`PrimitiveComponent.SetMaterial` _craftghost _index "/Game/Blueprint/Craft_Test/Material/MAT_GreenColor.MAT_GreenColor")
      (else
        (`PrimitiveComponent.SetMaterial` _craftghost _index "/Game/Blueprint/Build/Material/MAT_RedColor.MAT_RedColor"))))
  (`SceneComponent.K2_SetWorldTransform` (`self.CraftGhost`) (`self.CraftTransform`) false false))

(fn `SpawnCraft`
  (bind (_output_name _output_mesh _output_tracechannel _output_actor _output_resource) (break `/Game/Blueprint/Craft_Test/Crafting/ST_Crafting` (`|GetArrayItem` (`self.Craftable`) (`self.CraftID`))))
  (bind _returnvalue (`|SpawnActorFromClass` _output_actor (`self.CraftTransform`) "Undefined" "MultiplyWithRoot" null null))
  (message `/Game/Blueprint/Craft_Test/Crafting/BPI_CraftingInterface.SetCraftCost` _returnvalue _output_resource)
  (message `/Game/Blueprint/Craft_Test/Crafting/BPI_CraftingInterface.SetMesh` _returnvalue _output_mesh))

(fn `SpawnCraftGhost`
  (bind (_output_name _output_mesh) (break `/Game/Blueprint/Craft_Test/Crafting/ST_Crafting` (`|GetArrayItem` (`self.Craftable`) (`self.CraftID`))))
  (bind _returnvalue (`|AddComponentByClass` (`self.Player`) "/Script/Engine.StaticMeshComponent" false (`self.CraftTransform`)))
  (bind _output_get (set `self.CraftGhost` _returnvalue))
  (`StaticMeshComponent.SetStaticMesh` _output_get _output_mesh)
  (`PrimitiveComponent.SetCollisionEnabled` (`self.CraftGhost`) "NoCollision"))