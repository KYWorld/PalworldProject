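; Wooden box that acts as an interactable container with its own inventory.
; Interacting passes its InventorySystem to the player controller's PlayerMenu to show the container UI.
; LookAt sets the Korean prompt "열기" (Open) on its W_DisplayInfo widget.
; SetVisibilityWidget feeds its input straight into the widget's hidden-in-game flag, so true hides the prompt.
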(event `/Game/Blueprint/Component/Inventory/IInteractInterface.InteractWith`
  (params (PlayerCharacter :type "/Game/Blueprint/Character/Player/BP_PlayerCharacter Object Reference"))
  (bind _asbp_player_controller (cast `/Game/Blueprint/Character/Player/Controller/BP_PlayerController` (`GameplayStatics.GetPlayerController` 0)))
  (`/Game/Blueprint/Component/Inventory/UI/Base/W_DisplayMenu.ShowContainer` (`/Game/Blueprint/Character/Player/Controller/BP_PlayerController.PlayerMenu` _asbp_player_controller) (`self.InventorySystem`)))

(fn `LookAt`
  (returns (Message :type Text))
  (bind _asw_display_info (cast `/Game/Blueprint/Component/Inventory/UI/Base/W_DisplayInfo` (`WidgetComponent.GetWidget` (`self.Widget`))))
  (`/Game/Blueprint/Component/Inventory/UI/Base/W_DisplayInfo.ShowMessage` _asw_display_info "열기")
  (return ""))

(fn `Set Visibility Widget`
  (params (Result :type Boolean))
  (returns (NewParam :type Boolean))
  (`SceneComponent.SetHiddenInGame` (`self.Widget`) Result false)
  (return false))

(fn `UserConstructionScript`)