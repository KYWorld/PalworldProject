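; BP_CraftMaster is a base craftable structure that the player builds in place through an interaction.
; Setting its mesh stores the original materials, applies the MI_ObjectHeight material and limits collision to Visibility.
; Interacting locks player movement, plays an architecture montage and drives a timeline that animates the height gradient, then restores materials and full collision.
; Releasing stops the build; helpers expose two craft boxes and a message widget.
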(event `self.ReceiveBeginPlay`
  (bind _asbp_player_character (cast `/Game/Blueprint/Character/Player/BP_PlayerCharacter` (`GameplayStatics.GetPlayerCharacter` 0)))
  (set `self.Player` _asbp_player_character))

(event `/Game/Blueprint/Craft/Crafting/BPI_CraftingInterface.SetCraftMesh`
  (params (CraftMesh :type "StaticMesh Object Reference"))
  (bind _craft (`self.Craft`))
  (bind _returnvalue (`MeshComponent.GetMaterials` (`self.Craft`)))
  (`StaticMeshComponent.SetStaticMesh` (`self.Craft`) CraftMesh)
  (set `self.Materials` _returnvalue)
  (for (_ _array_index) _returnvalue
    (`PrimitiveComponent.SetMaterial` _craft _array_index "/Game/Blueprint/Craft/Material/MI_ObjectHeight.MI_ObjectHeight")
    (if (not (`self.IsCraftFinished`))
      (`/Engine/EditorBlueprintResources/StandardMacros.IncrementInt` (`self.ResourcesPlaced`)
        (:`  `
          (if (== (`self.Cost`) (`self.ResourcesPlaced`))
            (set `self.IsCraftFinished` true))))))
  (`PrimitiveComponent.SetCollisionResponseToAllChannels` _craft "ECR_Ignore")
  (`PrimitiveComponent.SetCollisionResponseToChannel` _craft "ECC_Visibility" "ECR_Block"))

(event `/Game/Blueprint/Craft/Crafting/BPI_CraftingInterface.SetCraftCost`
  (params (Resource :type Integer))
  (set `self.Cost` Resource))

(event `/Game/Blueprint/Craft/Crafting/BPI_CraftingInterface.InteractWithCraft`
  (params (IsTrigger :type Boolean))
  (bind _craft (`self.Craft`))
  (if IsTrigger
    (`CharacterMovementComponent.DisableMovement` (`Character.CharacterMovement` (`self.Player`)))
    (`|PlayMontage` (`Character.Mesh` (`self.Player`)) "/Game/Blueprint/Character/Player/Animation/Montage/Architecture/AM_Player_Architecture.AM_Player_Architecture"
      (:`then`
        (bind (_direction _gradient) (`Timeline|GradientTimeline` :!label _label)
          (:`Update`
            (`MeshComponent.SetScalarParameterValueOnMaterials` _craft "Gradient_Offset" (`KismetMathLibrary.Lerp` (`self.Min`) (`self.Max`) _gradient)))
          (:`Finished`
            (`Character.StopAnimMontage` (`self.Player`) "/Game/Blueprint/Character/Player/Animation/Montage/Architecture/AM_Player_Architecture.AM_Player_Architecture")
            (for (_array_element _array_index) (`self.Materials`)
              (set `self.IsCompletion` false)
              (`PrimitiveComponent.SetMaterial` _craft _array_index _array_element))
            (set `self.IsCompletion` true)
            (`self.SetText`)
            (set `self.ItemState` "NewEnumerator0")
            (`PrimitiveComponent.SetCollisionResponseToAllChannels` _craft "ECR_Block")
            (`PrimitiveComponent.SetCollisionResponseToChannel` _craft "ECC_Visibility" "ECR_Block")))))
    (else
      (`CharacterMovementComponent.SetMovementMode` (`Character.CharacterMovement` (`self.Player`)) "MOVE_Walking" 0)
      (`Character.StopAnimMontage` (`self.Player`) "/Game/Blueprint/Character/Player/Animation/Montage/Architecture/AM_Player_Architecture.AM_Player_Architecture")
      (goto _label :!via `Stop`))))

(event `/Game/Blueprint/Component/Inventory/IInteractInterface.InteractWith`
  (params (PlayerCharacter :type "/Game/Blueprint/Character/Player/BP_PlayerCharacter Object Reference")))

(fn `LookAt`
  (returns (Message :type Text))
  (bind _asw_display_info (cast `/Game/Blueprint/Component/Inventory/UI/Base/W_DisplayInfo` (`WidgetComponent.GetWidget` (`self.Widget`))))
  (`/Game/Blueprint/Component/Inventory/UI/Base/W_DisplayInfo.ShowMessage` _asw_display_info (`self.Message`))
  (return ""))

(fn `ReturnCraftBoxes`
  (returns (Boxes :type "Array of BoxComponent Object Reference"))
  (return (`|MakeArray` (`self.CraftBox1`) (`self.CraftBox2`))))

(fn `Set Visibility Widget`
  (params (Result :type Boolean))
  (returns (NewParam :type Boolean))
  (`SceneComponent.SetHiddenInGame` (`self.Widget`) Result false)
  (return false))

(fn `SetText`)

(fn `UserConstructionScript`)